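; LobbyGM is the multiplayer lobby game mode that tracks joining players and launches the match.
; On PostLogin, the server stores each controller and has its LobbyPC set up the menu with the GameInfoInstance server name and game time.
; It rebuilds the player-settings list and pushes it to every controller, as it does with game-time changes.
; LaunchTheGame server-travels to the RunForrestRun map, while SwapCharacter is an empty stub.
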(event `self.K2_PostLogin`
  (params (NewPlayer :type "PlayerController Object Reference"))
  (`/Engine/EditorBlueprintResources/ActorMacros.Switch Has Authority`
    (:`Authority`
      (`KismetArrayLibrary.Array_Add` (`self.PlayersController`) NewPlayer)
      (bind _asgame_info_instance (cast `/Game/Blueprints/AllLevels/GameInfoInstance` (`GameplayStatics.GetGameInstance`)))
      (bind _output_get (set `self.ServerName` (`/Game/Blueprints/AllLevels/GameInfoInstance.ServerName` _asgame_info_instance)))
      (bind _aslobby_pc (cast `/Game/Blueprints/Lobby/LobbyPC` NewPlayer))
      (`/Game/Blueprints/Lobby/LobbyPC.InitialSetup` _aslobby_pc)
      (`/Game/Blueprints/Lobby/LobbyPC.SetupLobbyMenu` _aslobby_pc _output_get)
      (`/Game/Blueprints/Lobby/LobbyPC.UpdateGameSetting` _aslobby_pc (`self.TimeOfASingleGame`))
      (`self.UpDateAll`))))

(event `UpDateAll`
  (bind _playerscontroller (`self.PlayersController`))
  (bind _output_get (set `self.CurrentPlayers` (`KismetArrayLibrary.Array_Length` (`self.PlayersController`))))
  (if (> _output_get 0)
    (`KismetArrayLibrary.Array_Clear` (`self.ConnectedPlayersInfo`))
    (for _array_element _playerscontroller
      (bind _aslobby_pc (cast `/Game/Blueprints/Lobby/LobbyPC` _array_element))
      (`KismetArrayLibrary.Array_Add` (`self.ConnectedPlayersInfo`) (`/Game/Blueprints/Lobby/LobbyPC.PlayerSetting` _aslobby_pc)))
    (for _array_element_2 _playerscontroller
      (bind _aslobby_pc_2 (cast `/Game/Blueprints/Lobby/LobbyPC` _array_element_2))
      (`/Game/Blueprints/Lobby/LobbyPC.AddPlayerInfo` _aslobby_pc_2 (`self.ConnectedPlayersInfo`)))))

(event `ServerUpdateSetting`
  (params (TimeOfSingleGame :type Integer))
  (bind _output_get (set `self.TimeOfASingleGame` TimeOfSingleGame))
  (for _array_element (`self.PlayersController`)
    (bind _aslobby_pc (cast `/Game/Blueprints/Lobby/LobbyPC` _array_element))
    (`/Game/Blueprints/Lobby/LobbyPC.UpdateGameSetting` _aslobby_pc _output_get)))

(event `LaunchTheGame`
  (`KismetSystemLibrary.ExecuteConsoleCommand` "servertravel/Game/Maps/RunForrestRun" null))

(event `SwapCharacter`
  (params (PlayerController :type "PlayerController Object Reference") (CharacterClass :type "Character Class Reference") (ChangedStatus :type Boolean)))

(fn `UserConstructionScript`)
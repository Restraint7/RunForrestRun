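; Game instance that manages menu flow and online sessions for hosting and joining multiplayer games.
; A save-game check opens the main menu or the options menu, and most widgets are cached for reuse.
; Hosting creates a session and opens Lobby as a listen server, while joining uses a search result, both behind a loading screen.
; Failures route to DisplayErrorMessage, which is an empty stub, and both error-to-string helpers return empty text.
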(event `SaveGameCheck`
  ;[1 1 1] Check For Save Game
  (bind _returnvalue (`GameplayStatics.DoesSaveGameExist` (`self.PlayerSettingsSave`)))
  (if _returnvalue
    (`self.ShowMainMenu`)
    (set `self.CreatedSaveFile` true)
    (else
      (`self.ShowOptionsMenu`)
      (set `PlayerController.bShowMouseCursor` true (`GameplayStatics.GetPlayerController` 0)))))

(event `self.HandleNetworkError`
  (params (FailureType :type "ENetworkFailure Enum" :default "NetDriverAlreadyExists") (bIsServer :type Boolean))
  ;[1 1 1] Handle network error
  (if bIsServer
    _
    (else
      _))
  (`self.DisplayErrorMessage` (`self.NetErrorToString` FailureType)))

(event `ShowMainMenu`
  (bind _returnvalue (`GameplayStatics.GetPlayerController` 0))
  ;[1 1 1] Show Main Menu and show cursor
  (`/Engine/EditorBlueprintResources/StandardMacros.IsValid` (`self.MainMenuWB`)
    (:`Is Valid`
      _)
    (:`Is Not Valid`
      (bind _returnvalue_2 (`|CreateWidget` "/Game/UI/MainMenu/MainMenu.MainMenu_C" _returnvalue))
      (set `self.MainMenuWB` _returnvalue_2)))
  (`UserWidget.AddToViewport` (`self.MainMenuWB`) 0)
  (set `PlayerController.bShowMouseCursor` true _returnvalue))

(event `ShowLoadingScreen`
  ;[1 1 1] Show LoadingScreen
  (`/Engine/EditorBlueprintResources/StandardMacros.IsValid` (`self.LoadingScreenWB`)
    (:`Is Valid`
      _)
    (:`Is Not Valid`
      (bind _returnvalue (`|CreateWidget` "/Game/UI/MainMenu/LoadingScreen.LoadingScreen_C" (`GameplayStatics.GetPlayerController` 0)))
      (set `self.LoadingScreenWB` _returnvalue)))
  (`UserWidget.AddToViewport` (`self.LoadingScreenWB`) 0))

(event `self.HandleTravelError`
  (params (FailureType :type "ETravelFailure Enum" :default "NoLevel"))
  ;[1 1 1] handel travel error
  (`self.DisplayErrorMessage` (`self.TravelErrorToString` FailureType)))

(event `ShowHostMenu`
  ;[1 1 1] Host Menu
  (`/Engine/EditorBlueprintResources/StandardMacros.IsValid` (`self.HostMenuWB`)
    (:`Is Valid`
      _)
    (:`Is Not Valid`
      (bind _returnvalue (`|CreateWidget` "/Game/UI/MainMenu/HostMenu.HostMenu_C" (`GameplayStatics.GetPlayerController` 0)))
      (set `self.HostMenuWB` _returnvalue)))
  (`UserWidget.AddToViewport` (`self.HostMenuWB`) 0))

(event `LaunchLobby`
  (params (ServerName :type Text))
  ;[1 1 1] launch lobby
  (set `self.ServerName` ServerName)
  (`self.ShowLoadingScreen`)
  (`CreateSessionCallbackProxy.CreateSession` (`GameplayStatics.GetPlayerController` 0) 8
    (:`OnSuccess`
      (`GameplayStatics.OpenLevel` "Lobby" true "listen"))
    (:`OnFailure`
      (`self.DisplayErrorMessage` "Failed to create session. Please try again."))))

(event `DestroySessionCaller`
  (params (PlayerController :type "PlayerController Object Reference"))
  ;[1 1 1] Destroy session
  (`DestroySessionCallbackProxy.DestroySession` PlayerController))

(event `ShowServerMenu`
  ;[1 1 1] Show Server Menu
  (bind _returnvalue (`|CreateWidget` "/Game/UI/MainMenu/ServerMenu.ServerMenu_C" (`GameplayStatics.GetPlayerController` 0)))
  (`UserWidget.AddToViewport` _returnvalue 0))

(event `JoinServer`
  (params (SessionToJoin :type "BlueprintSessionResult Structure"))
  ;[1 1 1] Join server
  (`self.ShowLoadingScreen`)
  (`JoinSessionCallbackProxy.JoinSession` (`GameplayStatics.GetPlayerController` 0) SessionToJoin
    (:`OnFailure`
      (`self.DisplayErrorMessage` "Failed to join session. Please try again."))))

(event `ShowOptionsMenu`
  (`/Engine/EditorBlueprintResources/StandardMacros.IsValid` (`self.OptionMenuWB`)
    (:`Is Valid`
      _)
    (:`Is Not Valid`
      (bind _returnvalue (`|CreateWidget` "/Game/UI/MainMenu/OptionMenu.OptionMenu_C"))
      (set `self.OptionMenuWB` _returnvalue)))
  (`UserWidget.AddToViewport` (`self.OptionMenuWB`) 0))

(fn `NetErrorToString`
  (params (FailureType :type "ENetworkFailure Enum" :default "NetDriverAlreadyExists"))
  (returns (OutString :type String))
  (return ""))

(fn `TravelErrorToString`
  (params (FailureType :type "ETravelFailure Enum" :default "NoLevel"))
  (returns (OutString :type String))
  (return ""))